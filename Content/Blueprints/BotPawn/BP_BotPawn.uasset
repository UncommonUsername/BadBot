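; BP_BotPawn is a player-controlled flying bot pawn that moves freely in three axes and fires twin blaster turrets.
; Enhanced Input drives look and movement, with movement vectors built from control rotation and fed to a FloatingPawnMovement component.
; Each tick the bot mesh snaps to the control rotation.
; Firing alternates left and right turret sockets via FlipFlop, spawning a beam actor and Niagara burst at each socket.
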(event Input|EnhancedActionEvents|EnhancedInputActionIA_Fire
  (params (ActionValue :type Boolean) (ElapsedSeconds :type Float%20%28double-precision%29) (TriggeredSeconds :type Float%20%28double-precision%29) (InputAction :type Input%20Action%20Object%20Reference :default "/Game/Blueprints/Input/InputActions/IA_Fire.IA_Fire"))
  (:Triggered
    (CallFunction|HandleFireTurrets)))

(event Input|EnhancedActionEvents|EnhancedInputActionIA_Look
  (params (ActionValue :type Vector%202D%20Structure) (ElapsedSeconds :type Float%20%28double-precision%29) (TriggeredSeconds :type Float%20%28double-precision%29) (InputAction :type Input%20Action%20Object%20Reference :default "/Game/Blueprints/Input/InputActions/IA_Look.IA_Look"))
  (:Triggered
    (CallFunction|HandleCameraMovement ActionValue)))

(event Input|EnhancedActionEvents|EnhancedInputActionIA_Move
  (params (ActionValue :type Vector :default "0, 0, 0") (ElapsedSeconds :type Float%20%28double-precision%29) (TriggeredSeconds :type Float%20%28double-precision%29) (InputAction :type Input%20Action%20Object%20Reference :default "/Game/Blueprints/Input/InputActions/IA_Move.IA_Move"))
  (:Triggered
    (CallFunction|HandleFloatingPawnMovement)))

(event EventBeginPlay
  (CallFunction|AddInputMappingContext))

(event EventTick
  (params (DeltaSeconds :type Float%20%28single-precision%29))
  (CallFunction|RotateMeshtoController))

(fn ConstructionScript)

(fn FireTurret
  (params (SocketName :type Name))
  (bind _botmesh (Variables|Default|GetBotMesh))
  (bind _returnvalue (Transformation|GetSocketTransform _botmesh SocketName "RTS_World"))
  (Game|SpawnActorfromClass "/Game/Blueprints/BlasterBeam/BP_BlasterBeam.BP_BlasterBeam_C" (Transformation|GetSocketTransform (Variables|Default|GetBotMesh) SocketName "RTS_World") "Undefined" "MultiplyWithRoot" 0 0 0)
  (Niagara|SpawnSystematLocation "/Game/FX/NS_BeamBurst.NS_BeamBurst" (.location _returnvalue) (.rotation _returnvalue)))

(fn GetLeftRightInputVector
  (return (* (Math|Vector|GetRightVector (Pawn|GetControlRotation :!class /Script/Engine.Pawn)) (.X (Math|Vector|BreakVector (Input|EnhancedActionValues|GetIA_Move))))))

(fn GetForwardBackwardInputVector
  (return (* (Math|Vector|GetForwardVector (Pawn|GetControlRotation :!class /Script/Engine.Pawn)) (.Y (Math|Vector|BreakVector (Input|EnhancedActionValues|GetIA_Move))))))

(fn HandleFloatingPawnMovement
  (Class|PawnMovementComponent|AddInputVector (Variables|Default|GetFloatingPawnMovement) (CallFunction|GetLeftRightInputVector) false)
  (Class|PawnMovementComponent|AddInputVector (Variables|Default|GetFloatingPawnMovement) (CallFunction|GetForwardBackwardInputVector) false)
  (Class|PawnMovementComponent|AddInputVector (Variables|Default|GetFloatingPawnMovement) (CallFunction|GetUpInputVector) false))

(fn HandleCameraMovement
  (params (Action%20Value :type Vector%202D%20Structure))
  (bind (_x _y) (Math|Vector2D|BreakVector2D Action%20Value))
  (Pawn|Input|AddControllerYawInput _x)
  (Pawn|Input|AddControllerPitchInput _y))

(fn HandleFireTurrets
  (Utilities|FlowControl|FlipFlop
    (:A
      (CallFunction|FireTurret (Variables|Default|Getturret_name_l)))
    (:B
      (CallFunction|FireTurret (Variables|Default|Getturret_name_r)))))

(fn RotateMeshtoController
  (Transformation|SetWorldRotation (Variables|Default|GetBotMesh) (Pawn|GetControlRotation :!class /Script/Engine.Pawn) false false))

(fn AddInputMappingContext
  (bind _asplayer_controller (Utilities|Casting|CastToPlayerController (Pawn|GetController)))
  (Input|AddMappingContext (PlayerController|LocalPlayerSubsystems|GetEnhancedInputLocalPlayerSubsystem _asplayer_controller) "/Game/Blueprints/Input/IMC_Bot.IMC_Bot" 0 "(bIgnoreAllPressedKeysUntilRelease=True,bForceImmediately=False)"))

(fn GetUpInputVector
  (return (* (Math|Vector|GetUpVector (Pawn|GetControlRotation :!class /Script/Engine.Pawn)) (.Z (Math|Vector|BreakVector (Input|EnhancedActionValues|GetIA_Move))))))