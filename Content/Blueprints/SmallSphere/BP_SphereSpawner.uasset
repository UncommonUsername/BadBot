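; BP_SphereSpawner is an actor that keeps spawning BP_SmallSphere actors around itself.
; On BeginPlay it starts a looping timer at SphereSpawnTime intervals that fires the SpawnSphere event.
; Each spawn gets a random rotation and a location from GetRandomPointInRadius, which offsets the spawner's position along a random direction by a random distance up to SpawnRadius.
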(event Custom|SpawnSphere
  ;[1 0.9283 0.1475] Sphere Spawner
  (Game|SpawnActorfromClass "/Game/Blueprints/SmallSphere/BP_SmallSphere.BP_SmallSphere_C" (Math|Transform|MakeTransform (CallFunction|GetRandomPointinRadius) (Math|Random|RandomRotator false) "1.000000,1.000000,1.000000") "Undefined" "MultiplyWithRoot" 0 0))

(event EventBeginPlay
  ;[1 0.9283 0.1475] Sphere Spawner
  (Utilities|Time|SetTimerbyEvent (delegate Custom|SpawnSphere) (Variables|Default|Getsphere_spawn_time) true))

(event EventTick
  (params (DeltaSeconds :type Float%20%28single-precision%29)))

(fn ConstructionScript)

(fn GetRandomPointinRadius
  (return (+ (Transformation|GetActorLocation) (* (Math|Vector|GetForwardVector (Math|Random|RandomRotator false)) (Math|Random|RandomFloatinRange 0.0 (Variables|Default|Getspawn_radius))))))