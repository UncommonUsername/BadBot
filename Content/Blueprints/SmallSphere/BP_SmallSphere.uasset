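; BP_SmallSphere is a short-lived actor that wanders through the world and winks out when its lifetime expires.
; Each tick it moves along its forward vector at Velocity without sweeping, then adds a scaled random rotation, so its heading drifts erratically.
; A timer set at BeginPlay fires WinkOut, whose timeline drives the mesh's uniform world scale through BlinkSphere and destroys the actor when finished.
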(event Custom|WinkOut
  (bind _scale (Timeline|WinkOutTimeline Play)
    (:Update
      (CallFunction|BlinkSphere _scale))
    (:Finished
      (Actor|DestroyActor))))

(event EventBeginPlay
  (Utilities|Time|SetTimerbyEvent (delegate Custom|WinkOut) (Variables|Default|GetLifetime)))

(event EventTick
  (params (DeltaSeconds :type Float%20%28single-precision%29))
  (CallFunction|UpdateMovement DeltaSeconds)
  (CallFunction|UpdateRotation))

(fn ConstructionScript)

(fn UpdateRotation
  (Class|Actor|AddActorWorldRotation (* (* (Math|Random|RandomRotator false) (Variables|Default|Getrandom_rotator_scale_factor)) (Utilities|Time|GetWorldDeltaSeconds))))

(fn UpdateMovement
  (params (DeltaTime :type Float%20%28single-precision%29))
  (Transformation|AddActorWorldOffset (* DeltaTime (* (Transformation|GetActorForwardVector) (Variables|Default|Getvelocity)))))

(fn BlinkSphere
  (params (InputPin :type Float%20%28single-precision%29))
  (Transformation|SetWorldScale3D (Variables|Default|GetSphereMesh) (Math|Vector|MakeVector InputPin InputPin InputPin)))